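; BP_SB_MoveForwardReturnIsDeadTest is a functional test that checks the side-scroller player character dies when moved along a set direction.
; StartTest caches player character 0, then Tick feeds it movement input along the WhereToGo vector every frame.
; Each tick it casts to BP_SideScrollerCharacter and finishes as Succeeded once IsDead is true.
; The graph has no explicit failure branch.
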(event `self.ReceiveStartTest`
  (set `self.Character` (`GameplayStatics.GetPlayerCharacter` 0)))

(event `self.ReceiveTick`
  (params (DeltaSeconds :type "Float (single-precision)"))
  (bind _character (`self.Character`))
  (`Pawn.AddMovementInput` _character (`self.WhereToGo`) 1.0 false)
  (bind _asbp_side_scroller_character (cast `/Game/SideScrollerBP/Blueprints/Character/BP_SideScrollerCharacter` _character))
  (if (`/Game/SideScrollerBP/Blueprints/Character/BP_SideScrollerCharacter.Is_dead` _asbp_side_scroller_character)
    (`self.FinishTest` "Succeeded")))

(fn `UserConstructionScript`)