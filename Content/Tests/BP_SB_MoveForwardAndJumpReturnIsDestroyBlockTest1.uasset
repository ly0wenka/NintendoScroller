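; BP_SB_MoveForwardAndJumpReturnIsDestroyBlockTest1 is a functional test that drives the player character in a side-scroller until it dies.
; StartTest caches and prints player character 0, then Tick feeds it movement input along WhereToGo and calls Jump every frame.
; The test succeeds once BP_SideScrollerCharacter reports IsDead; despite its name, it never checks block destruction directly and has no explicit failure branch.
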(event `self.ReceiveStartTest`
  (bind _output_get (set `self.Character` (`GameplayStatics.GetPlayerCharacter` 0)))
  (`KismetSystemLibrary.PrintString` (`KismetSystemLibrary.GetDisplayName` _output_get)))

(event `self.ReceiveTick`
  (params (DeltaSeconds :type "Float (single-precision)"))
  (bind _character (`self.Character`))
  (`Pawn.AddMovementInput` _character (`self.WhereToGo`) 1.0 false)
  (`Character.Jump` _character)
  (bind _asbp_side_scroller_character (cast `/Game/SideScrollerBP/Blueprints/Character/BP_SideScrollerCharacter` _character)
    (:`then`
      (if (`/Game/SideScrollerBP/Blueprints/Character/BP_SideScrollerCharacter.Is_dead` _asbp_side_scroller_character)
        (`self.FinishTest` "Succeeded")))
    (:`CastFailed`
      (`KismetSystemLibrary.PrintString` "CastFailed"))))

(fn `UserConstructionScript`)